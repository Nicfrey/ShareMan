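; Enemy character that reflects its detection and chase state through UI, movement speed and highlighting.
; Events drive the looking bar and exclamation/question marks in its WBP_UIEnemy widget, and switch walk speed for chasing.
; Spotted enables custom depth on the mesh until a timer, polled on Tick, finishes.
; Player death and revive events update blackboard flags, and the construction script defaults empty patrol positions to the actor's location.
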(event Custom|ChangeLookingUI
  (params (Percentage :type Float%20%28double-precision%29))
  (bind _aswbp_uienemy (Utilities|Casting|CastToWBP_UIEnemy (UserInterface|GetUserWidgetObject (Variables|Default|GetWidget))))
  (Default|SetVisibilityLookingBar _aswbp_uienemy Percentage))

(event Custom|ChangeSpeed
  (params (ChasePlayer :type Boolean))
  (bind _charactermovement (Variables|Character|GetCharacterMovement))
  (if ChasePlayer
    (Variables|/Script/Engine.CharacterMovementComponent|SetMaxWalkSpeed _charactermovement (Variables|Default|GetTargetSpeed))
    (else
      (Variables|/Script/Engine.CharacterMovementComponent|SetMaxWalkSpeed _charactermovement (Variables|Default|GetNormalSpeed)))))

(event Custom|ChangeChaseUI
  (params (BeginChase :type Boolean) (BeginAfterChase :type Boolean))
  (bind _widget (Variables|Default|GetWidget))
  (bind _widget_2 (Variables|Default|GetWidget))
  (bind _returnvalue (UserInterface|GetUserWidgetObject _widget))
  (bind _returnvalue_2 (UserInterface|GetUserWidgetObject _widget_2))
  (if BeginChase
    (bind _aswbp_uienemy (Utilities|Casting|CastToWBP_UIEnemy _returnvalue_2))
    (Default|SetVisibilityExclamationMark _aswbp_uienemy true)
    (else
      (bind _aswbp_uienemy_2 (Utilities|Casting|CastToWBP_UIEnemy _returnvalue_2))
      (Default|SetVisibilityExclamationMark _aswbp_uienemy_2 false)))
  (if BeginAfterChase
    (bind _aswbp_uienemy_3 (Utilities|Casting|CastToWBP_UIEnemy _returnvalue))
    (Default|SetVisibilityQuestionMark _aswbp_uienemy_3 true)
    (else
      (bind _aswbp_uienemy_4 (Utilities|Casting|CastToWBP_UIEnemy _returnvalue))
      (Default|SetVisibilityQuestionMark _aswbp_uienemy_4 false))))

(event Custom|Spotted
  (bind _visibletimer (Variables|Default|GetVisibleTimer))
  (Rendering|SetRenderCustomDepth (Variables|Character|GetMesh) true)
  (Default|ResetTimer _visibletimer)
  (Default|StartTimer _visibletimer))

(event Custom|OnPlayerDead
  (bind _returnvalue (Pawn|GetController))
  (bind _returnvalue_2 (AI|GetBlackboard _returnvalue))
  (AI|Components|Blackboard|SetValueasBool _returnvalue_2 (Utilities|Name|MakeLiteralName "IsChasingPlayer") false)
  (AI|Components|Blackboard|SetValueasBool _returnvalue_2 (Utilities|Name|MakeLiteralName "IsPlayerDead") true)
  (CallFunction|ChangeSpeed false)
  (CallFunction|ChangeChaseUI false false))

(event Custom|OnPlayerRevive
  (AI|Components|Blackboard|SetValueasBool (AI|GetBlackboard (Pawn|GetController)) (Utilities|Name|MakeLiteralName "IsPlayerDead") false))

(event EventBeginPlay
  (|CallParentFunction))

(event Collision|EventActorBeginOverlap
  (params (OtherActor :type Actor%20Object%20Reference))
  (|CallParentFunction OtherActor) ; This node is disabled and will not be called.\nDrag off pins to build functionality.
)

(event EventTick
  (params (DeltaSeconds :type Float%20%28single-precision%29))
  (|CallParentFunction DeltaSeconds)
  (if (Variables|/Game/Blueprints/InteractableItem/BPC_Timer.BPC_Timer_C|Getstarted (Variables|Default|GetVisibleTimer))
    (if (Default|HasFinished (Variables|Default|GetVisibleTimer))
      (Default|ResetTimer (Variables|Default|GetVisibleTimer))
      (Rendering|SetRenderCustomDepth (Variables|Character|GetMesh) false))))

(fn ConstructionScript
  (|CallParentFunction)
  (if (== (Utilities|Array|Length (Variables|Default|GetPatrolPositions)) 0)
    (Utilities|Array|Add (Variables|Default|GetPatrolPositions) (Transformation|GetActorLocation))))
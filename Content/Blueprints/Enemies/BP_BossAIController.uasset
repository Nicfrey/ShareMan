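; AI controller for a boss enemy whose behavior depends on whether a referenced light is on.
; While the light is on, sight perception updates for the player set the controlled BP_EnemyCharacter's Status and store the player's capsule position as LastSeenPlayerPosition.
; MoveToLightLever and MovetoHide share identical logic: while the light is off, each moves the pawn to the light actor.
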(event OnTargetPerceptionUpdated(AIPerception)
  (params (Actor :type Actor%20Object%20Reference) (Stimulus :type AI%20Stimulus%20Structure))
  (bind _returnvalue (Game|GetPlayerCharacter 0))
  (if (Default|IsLighton (Variables|Default|GetLightClass))
    (bind _returnvalue_2 (Class|AIPerceptionSystem|GetSenseClassforStimulus Stimulus))
    (if (== _returnvalue_2 "/Script/AIModule.AISense_Sight")
      (if (== _returnvalue Actor)
        (bind _asbp_enemy_character (Utilities|Casting|CastToBP_EnemyCharacter (Pawn|GetControlledPawn)))
        (Variables|/Game/Blueprints/Enemies/BP_EnemyCharacter.BP_EnemyCharacter_C|Setstatus _asbp_enemy_character "NewEnumerator0")
        (Variables|Default|SetLastSeenPlayerPosition (Transformation|GetWorldLocation (Variables|/Script/Engine.Character|GetCapsuleComponent _returnvalue)))))))

(event Custom|MoveToLightLever
  (bind _lightclass (Variables|Default|GetLightClass))
  (if (not (Default|IsLighton _lightclass))
    (AI|AIMoveTo (Pawn|GetControlledPawn) "0, 0, 0" _lightclass 5.0 false)))

(event EventMovetoHide
  (bind _lightclass (Variables|Default|GetLightClass))
  (if (not (Default|IsLighton _lightclass))
    (AI|AIMoveTo (Pawn|GetControlledPawn) "0, 0, 0" _lightclass 5.0 false)))

(event EventTick
  (params (DeltaSeconds :type Float%20%28single-precision%29))
  (|CallParentFunction DeltaSeconds))

(event EventBeginPlay
  (|CallParentFunction))

(fn ConstructionScript
  (|CallParentFunction))
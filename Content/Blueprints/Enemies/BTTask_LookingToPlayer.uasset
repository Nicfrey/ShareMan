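; Behavior tree task that runs an enemy's after-chase phase, showing the after-chase UI and managing the AI controller's post-chase timer.
; Each run starts the timer if needed and finishes successfully at once, without waiting.
; Once the timer expires, it restarts it, copies HasPlayerOnSight into IsChasingPlayer, records the player's current location as LastKnownPlayerLocation, updates speed and clears the chase UI.
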(event EventReceiveExecuteAI
  (params (OwnerController :type AI%20Controller%20Object%20Reference) (ControlledPawn :type Pawn%20Object%20Reference))
  (bind _asbp_enemy_character (Utilities|Casting|CastToBP_EnemyCharacter ControlledPawn))
  (Default|ChangeChaseUI _asbp_enemy_character false true)
  (bind _asbp_base_aicontroller (Utilities|Casting|CastToBP_BaseAIController OwnerController))
  (if (Default|AfterChaseTimerStarted _asbp_base_aicontroller)
    (if (Default|HasFinished (Variables|/Game/Blueprints/Enemies/BP_BaseAIController.BP_BaseAIController_C|GetTimerAfterChase _asbp_base_aicontroller))
      (Default|RestartTimer (Variables|/Game/Blueprints/Enemies/BP_BaseAIController.BP_BaseAIController_C|GetTimerAfterChase _asbp_base_aicontroller))
      (AI|Components|Blackboard|SetValueasBool (AI|GetBlackboard _asbp_base_aicontroller) (Utilities|Name|MakeLiteralName "IsChasingPlayer") (ScalableFloat|GetValueasBool (AI|GetBlackboard _asbp_base_aicontroller) (Utilities|Name|MakeLiteralName "HasPlayerOnSight")))
      (AI|Components|Blackboard|SetValueasVector (AI|GetBlackboard _asbp_base_aicontroller) (Utilities|Name|MakeLiteralName "LastKnownPlayerLocation") (Transformation|GetActorLocation (Game|GetPlayerCharacter 0)))
      (Default|ChangeSpeed _asbp_enemy_character (ScalableFloat|GetValueasBool (AI|GetBlackboard _asbp_base_aicontroller) (Utilities|Name|MakeLiteralName "HasPlayerOnSight")))
      (Default|ChangeChaseUI _asbp_enemy_character false false)
      (AI|BehaviorTree|FinishExecute true :!label _label)
      (else
        (AI|BehaviorTree|FinishExecute true)))
    (else
      (Default|StartTimer (Variables|/Game/Blueprints/Enemies/BP_BaseAIController.BP_BaseAIController_C|GetTimerAfterChase _asbp_base_aicontroller))
      (goto _label))))
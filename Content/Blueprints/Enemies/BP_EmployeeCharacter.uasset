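; BP_EmployeeCharacter is an enemy employee character whose walk speed depends on a hiding state.
; ChangeSpeedHiding sets the movement component's MaxWalkSpeed to MaxSpeedHide or NormalSpeed from its IsHiding flag, then prints the result as debug output.
; The event graph and construction script only defer to the parent, and nothing in this file calls the speed function.
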(event EventBeginPlay
  (|CallParentFunction) ; This node is disabled and will not be called.\nDrag off pins to build functionality.
)

(event Collision|EventActorBeginOverlap
  (params (OtherActor :type Actor%20Object%20Reference))
  (|CallParentFunction OtherActor) ; This node is disabled and will not be called.\nDrag off pins to build functionality.
)

(event EventTick
  (params (DeltaSeconds :type Float%20%28single-precision%29))
  (|CallParentFunction DeltaSeconds))

(fn ConstructionScript
  (|CallParentFunction))

(fn ChangeSpeedHiding
  (params (IsHiding :type Boolean))
  (bind _charactermovement (Variables|Character|GetCharacterMovement))
  (if IsHiding
    (Variables|/Script/Engine.CharacterMovementComponent|SetMaxWalkSpeed _charactermovement (Variables|Default|GetMaxSpeedHide))
    (else
      (Variables|/Script/Engine.CharacterMovementComponent|SetMaxWalkSpeed _charactermovement (Variables|Default|GetNormalSpeed))))
  (Development|PrintString (Utilities|String|ToString(Float) (Variables|/Script/Engine.CharacterMovementComponent|GetMaxWalkSpeed _charactermovement))))
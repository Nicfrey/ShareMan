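; Game mode that manages level flow, game-over state, sky lighting and background audio.
; On BeginPlay it caches the SkyLight, forces all scalability settings to lowest and starts ambient sound.
; A counter of chasing enemies swaps chase and ambient audio, while an event toggles sky intensity between default and night.
; ChangeLevel restarts FirstLevel, advances a won tutorial to it, and sends a lost tutorial or Playground to TutorialLevel.
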(event Custom|RemoveEnemyChasing
  (bind _audio (Variables|Default|GetAudio))
  (bind _result (Math|Integer|DecrementInt (Variables|Default|GetNbEnemyChasingPlayer))
    (:%20%20
      (if (== _result 0)
        (Audio|Components|Audio|SetSound _audio (Variables|Musics|GetAmbientSound))
        (Audio|Components|Audio|Play _audio 0.0)))))

(event Custom|ChangeSkyIntensity
  (params (IsLightOn :type Boolean))
  (bind _skylight (Variables|Default|GetSkyLight))
  (bind _lightcomponent (Variables|/Script/Engine.SkyLight|GetLightComponent _skylight))
  (if IsLightOn
    (Rendering|Components|Light|SetIntensity _lightcomponent (Variables|Default|GetDefaultIntensity))
    (else
      (Rendering|Components|Light|SetIntensity _lightcomponent (Variables|Default|GetNightIntensity)))))

(event Custom|ChangeLevel
  (params (hasWon :type Boolean))
  (bind _returnvalue (Game|GetCurrentLevelName true))
  (if (Utilities|Enum|Equal(Enum) _returnvalue "FirstLevel")
    (Game|OpenLevel(byName) "FirstLevel")
    (elif (Utilities|Enum|Equal(Enum) _returnvalue "TutorialLevel")
      (if hasWon
        (Game|OpenLevel(byName) "FirstLevel")
        (else
          (Game|OpenLevel(byName) "TutorialLevel" :!label _label)))
      (elif (Utilities|Enum|Equal(Enum) _returnvalue "Playground")
        (goto _label)))))

(event Custom|GameOver
  (Variables|Default|SetGameIsOver true))

(event Custom|AddEnemyChasing
  (bind _audio (Variables|Default|GetAudio))
  (bind _result (Math|Integer|IncrementInt (Variables|Default|GetNbEnemyChasingPlayer))
    (:%20%20
      (if (== _result 1)
        (Audio|Components|Audio|SetSound _audio (Variables|Musics|GetChaseSound))
        (Audio|Components|Audio|Play _audio 0.0)))))

(event EventBeginPlay
  (bind _audio (Variables|Default|GetAudio))
  (bind _returnvalue (Actor|GetActorOfClass "/Script/Engine.SkyLight"))
  (Variables|Default|SetSkyLight _returnvalue)
  (CallFunction|SetupGraphics)
  (Audio|Components|Audio|SetSound _audio (Variables|Musics|GetAmbientSound))
  (Audio|Components|Audio|Play _audio 0.0))

(event EventTick
  (params (DeltaSeconds :type Float%20%28single-precision%29)))

(fn ConstructionScript)

(fn GetPercentageShareGot
  (return (Math|Float|Round (* (/ 0.0 (Math|Conversions|ToFloat(Integer) 0)) 1e+02))))

(fn IsGameOver
  (return (Variables|Default|GetGameIsOver)))

(fn SetupGraphics
  (bind _returnvalue (Settings|GetGameUserSettings))
  (Utilities|FlowControl|Sequence
    (:then_0
      (Class|GameUserSettings|SetShadingQuality _returnvalue))
    (:then_1
      (Class|GameUserSettings|SetFoliageQuality _returnvalue))
    (:then_2
      (Class|GameUserSettings|SetVisualEffectQuality _returnvalue))
    (:then_3
      (Class|GameUserSettings|SetTextureQuality _returnvalue))
    (:then_4
      (Class|GameUserSettings|SetReflectionQuality _returnvalue))
    (:then_5
      (Class|GameUserSettings|SetGlobalIlluminationQuality _returnvalue))
    (:then_6
      (Class|GameUserSettings|SetShadowQuality _returnvalue))
    (:then_7
      (Class|GameUserSettings|SetPostProcessingQuality _returnvalue))
    (:then_8
      (Class|GameUserSettings|SetAntiAliasingQuality _returnvalue))
    (:then_9
      (Class|GameUserSettings|SetViewDistanceQuality _returnvalue))
    (:then_10
      (Class|GameUserSettings|ApplySettings _returnvalue true))))

(fn IsPlayerBeingChased
  (return (> (Variables|Default|GetNbEnemyChasingPlayer) 0)))

(fn PlayAmbientSound
  (bind _audio (Variables|Default|GetAudio))
  (Audio|Components|Audio|SetSound _audio (Variables|Musics|GetAmbientSound))
  (Audio|Components|Audio|Play _audio 0.0)
  (Variables|Default|SetNbEnemyChasingPlayer 0))
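; HUD_Menu is the menu HUD that owns and switches between the main menu and options screens.
; On BeginPlay it creates both widgets, stores references to them and shows the main menu.
; ChangeToOption and ChangeToMain clear all widgets from the viewport, then re-add the cached options or main menu widget, so the screens are reused rather than recreated.
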(event Custom|ChangeToOption
  (Viewport|RemoveAllWidgets)
  (UserInterface|Viewport|AddtoViewport (Variables|Default|GetOptionRef) 0))

(event Custom|ChangeToMain
  (Viewport|RemoveAllWidgets)
  (UserInterface|Viewport|AddtoViewport (Variables|Default|GetMainMenuRef) 0))

(event EventBeginPlay
  (bind _returnvalue (UserInterface|CreateWidget "/Game/Blueprints/HUDs/Menu/WBP_MainMenu.WBP_MainMenu_C"))
  (bind _output_get (Variables|Default|SetMainMenuRef _returnvalue))
  (UserInterface|Viewport|AddtoViewport _output_get 0)
  (bind _returnvalue_2 (UserInterface|CreateWidget "/Game/Blueprints/HUDs/Menu/WBP_Options.WBP_Options_C"))
  (Variables|Default|SetOptionRef _returnvalue_2))

(event Collision|EventActorBeginOverlap
  (params (OtherActor :type Actor%20Object%20Reference)))

(event EventTick
  (params (DeltaSeconds :type Float%20%28single-precision%29)))

(fn ConstructionScript)
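; Player HUD Blueprint that creates and manages the in-game HUD widget and the win/lose screen.
; On BeginPlay it creates both widgets and shows only the gameplay one.
; Its events forward percentage, interaction prompts, life, anger value, collected cards and advice updates to the gameplay widget.
; Two switch events swap between gameplay and end-game screens, passing the win result to the latter.
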(event Custom|ChangePercentageGot
  (params (Percentage :type Float%20%28double-precision%29))
  (Default|SetTextPercentage (Variables|Default|GetUi_Ref) Percentage))

(event Custom|ChangeTextHoldInteract
  (params (InteractText :type String))
  (Default|SetTextHoldInteract (Variables|Default|GetUi_Ref) InteractText))

(event Custom|ChangeVisibilityInteractText
  (params (IsVisible :type Boolean))
  (Default|HideTextInteract (Variables|Default|GetUi_Ref) IsVisible))

(event Custom|UpdateLife
  (params (Life :type Integer))
  (Default|UpdateLifeHUD (Variables|Default|GetUi_Ref) Life))

(event Custom|UpdateAngryValue
  (params (Percentage :type Float%20%28double-precision%29))
  (Default|UpdateTriggerProgress (Variables|Default|GetUi_Ref) Percentage))

(event Custom|SwitchUIEndGame
  (params (hasWon :type Boolean))
  (bind _ui_endgame (Variables|Default|GetUI_EndGame))
  (UserInterface|Viewport|AddtoViewport _ui_endgame 0)
  (Widget|RemovefromParent (Variables|Default|GetUi_Ref))
  (Default|SetupHUD _ui_endgame hasWon))

(event Custom|SwitchUIGame
  (UserInterface|Viewport|AddtoViewport (Variables|Default|GetUi_Ref) 0)
  (Widget|RemovefromParent (Variables|Default|GetUI_EndGame)))

(event Custom|CardTaken
  (params (Color :type EColorDoor%20Enum :default "NewEnumerator0"))
  (Default|UpdateCard (Variables|Default|GetUi_Ref) Color))

(event Custom|ActivateAdvice
  (params (Advice :type String) (SecondAdvice :type String))
  (Default|ActivateAdvice (Variables|Default|GetUi_Ref) Advice SecondAdvice))

(event Custom|ChangeTextPressedInteract
  (params (InteractText :type String))
  (Default|SetTextPressedInteraction (Variables|Default|GetUi_Ref) InteractText))

(event EventBeginPlay
  (bind _returnvalue (UserInterface|CreateWidget "/Game/Blueprints/HUDs/WBP_HUDPlayer.WBP_HUDPlayer_C"))
  (bind _output_get (Variables|Default|SetUi_Ref _returnvalue))
  (UserInterface|Viewport|AddtoViewport _output_get 0)
  (bind _returnvalue_2 (UserInterface|CreateWidget "/Game/Blueprints/HUDs/WBP_HUDWinLose.WBP_HUDWinLose_C"))
  (Variables|Default|SetUI_EndGame _returnvalue_2))

(event Collision|EventActorBeginOverlap
  (params (OtherActor :type Actor%20Object%20Reference)))

(event EventTick
  (params (DeltaSeconds :type Float%20%28single-precision%29)))

(fn ConstructionScript)
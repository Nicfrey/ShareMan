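; BPC_ColorDoor is a component, by its name, that applies a door color to mesh materials.
; ApplyColorToMaterial switches on the Color value to set the Color and ColorEmissive parameters of a passed-in material instance, then assigns it to the given mesh slot.
; White is the exception, using black for ColorEmissive so it does not glow.
; A separate ApplyEmissiveScalar event sets the Emissive scalar to a fixed low value.
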(event Custom|ApplyEmissiveScalar
  (params (Material%20Instance :type Material%20Instance%20Dynamic%20Object%20Reference))
  (Rendering|Material|SetScalarParameterValue Material%20Instance "Emissive" 0.05 :!class /Script/Engine.MaterialInstanceDynamic))

(event Custom|ApplyColorToMaterial
  (params (Mesh :type Static%20Mesh%20Component%20Object%20Reference) (Material%20Instance :type Material%20Instance%20Dynamic%20Object%20Reference) (Material%20Index :type Integer))
  (bind _redvalue (Variables|Default|GetRedValue))
  (bind _bluevalue (Variables|Default|GetBlueValue))
  (bind _greenvalue (Variables|Default|GetGreenValue))
  (switch Utilities|FlowControl|Switch|SwitchonEColorDoor (Variables|Default|GetColor)
    (:NewEnumerator0
      (Rendering|Material|SetVectorParameterValue Material%20Instance "Color" _redvalue :!class /Script/Engine.MaterialInstanceDynamic)
      (Rendering|Material|SetVectorParameterValue Material%20Instance "ColorEmissive" _redvalue :!class /Script/Engine.MaterialInstanceDynamic))
    (:NewEnumerator1
      (Rendering|Material|SetVectorParameterValue Material%20Instance "Color" _bluevalue :!class /Script/Engine.MaterialInstanceDynamic)
      (Rendering|Material|SetVectorParameterValue Material%20Instance "ColorEmissive" _bluevalue :!class /Script/Engine.MaterialInstanceDynamic))
    (:NewEnumerator2
      (Rendering|Material|SetVectorParameterValue Material%20Instance "Color" _greenvalue :!class /Script/Engine.MaterialInstanceDynamic)
      (Rendering|Material|SetVectorParameterValue Material%20Instance "ColorEmissive" _greenvalue :!class /Script/Engine.MaterialInstanceDynamic))
    (:NewEnumerator3
      (Rendering|Material|SetVectorParameterValue Material%20Instance "Color" (Variables|Default|GetWhiteValue) :!class /Script/Engine.MaterialInstanceDynamic)
      (Rendering|Material|SetVectorParameterValue :self Material%20Instance :ParameterName "ColorEmissive" :!class /Script/Engine.MaterialInstanceDynamic)))
  (Rendering|Material|SetMaterial Mesh Material%20Index Material%20Instance))

(event EventBeginPlay)

(event EventTick
  (params (DeltaSeconds :type Float%20%28single-precision%29)))
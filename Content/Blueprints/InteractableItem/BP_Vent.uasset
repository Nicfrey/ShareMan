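; BP_Vent is an interactable hiding spot that lets the player character hide from enemies.
; Its box overlap registers and clears the vent as the player's current interact vent.
; Interact toggles the player's IsHidden state, switching movement, mesh visibility and the capsule's Pawn collision response.
; On hiding, it also finds every BP_EnemyCharacter and makes each lose sight of the player.
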(event OnComponentBeginOverlap(Box)
  (params (OverlappedComponent :type Primitive%20Component%20Object%20Reference) (OtherActor :type Actor%20Object%20Reference) (OtherComp :type Primitive%20Component%20Object%20Reference) (OtherBodyIndex :type Integer) (bFromSweep :type Boolean) (SweepResult :type Hit%20Result%20Structure%20%28by%20ref%29))
  (bind _asbp_player_character (Utilities|Casting|CastToBP_PlayerCharacter OtherActor))
  (Variables|/Game/Blueprints/Player/BP_PlayerCharacter.BP_PlayerCharacter_C|SetCurrentInteractVent _asbp_player_character self))

(event OnComponentEndOverlap(Box)
  (params (OverlappedComponent :type Primitive%20Component%20Object%20Reference) (OtherActor :type Actor%20Object%20Reference) (OtherComp :type Primitive%20Component%20Object%20Reference) (OtherBodyIndex :type Integer))
  (bind _asbp_player_character (Utilities|Casting|CastToBP_PlayerCharacter OtherActor))
  (Variables|/Game/Blueprints/Player/BP_PlayerCharacter.BP_PlayerCharacter_C|SetCurrentInteractVent _asbp_player_character 0))

(event EventBeginPlay)

(event Collision|EventActorBeginOverlap
  (params (OtherActor :type Actor%20Object%20Reference)))

(event EventTick
  (params (DeltaSeconds :type Float%20%28single-precision%29)))

(event EventInteract
  (bind _asbp_player_character (Utilities|Casting|CastToBP_PlayerCharacter (Game|GetPlayerCharacter 0)))
  (if (Variables|/Game/Blueprints/Player/BP_PlayerCharacter.BP_PlayerCharacter_C|GetIsHidden _asbp_player_character)
    (Pawn|Components|CharacterMovement|SetMovementMode (Variables|/Script/Engine.Character|GetCharacterMovement _asbp_player_character) "MOVE_Walking" 0)
    (Development|SetHiddeninGame (Variables|/Script/Engine.Character|GetMesh _asbp_player_character) false false)
    (Collision|SetCollisionResponsetoChannel (Variables|/Script/Engine.Character|GetCapsuleComponent _asbp_player_character) "ECC_Pawn" "ECR_Block")
    (Variables|/Game/Blueprints/Player/BP_PlayerCharacter.BP_PlayerCharacter_C|SetIsHidden _asbp_player_character false)
    (else
      (Pawn|Components|CharacterMovement|DisableMovement (Variables|/Script/Engine.Character|GetCharacterMovement _asbp_player_character))
      (Development|SetHiddeninGame (Variables|/Script/Engine.Character|GetMesh _asbp_player_character) true false)
      (Collision|SetCollisionResponsetoChannel (Variables|/Script/Engine.Character|GetCapsuleComponent _asbp_player_character) "ECC_Pawn" "ECR_Overlap")
      (Variables|/Game/Blueprints/Player/BP_PlayerCharacter.BP_PlayerCharacter_C|SetIsHidden _asbp_player_character true)
      (bind _outactors (Actor|GetAllActorsOfClass "/Game/Blueprints/Enemies/BP_EnemyCharacter.BP_EnemyCharacter_C"))
      (for _array_element _outactors
        (Default|LoseSightOfPlayer _array_element true)))))

(fn ConstructionScript)
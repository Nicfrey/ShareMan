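; Interactable camera actor, going by its folder, whose view is turned through a LookAround event.
; BeginPlay caches the camera's world rotation, and LookAround adds input X to roll and Z to yaw, zeroing pitch.
; The result is applied as relative rotation with roll and yaw angle-clamped, while the cached rotation itself stays unclamped.
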(event Custom|LookAround
  (params (Input :type Vector))
  (bind _output_get (Variables|Default|SetCurrentRotationCamera (Math|Rotator|MakeRotator (+ (.x Input) (.roll (Variables|Default|GetCurrentRotationCamera))) 0.0 (+ (.z Input) (.yaw (Variables|Default|GetCurrentRotationCamera))))))
  (Transformation|SetRelativeRotation (Variables|Default|GetCamera) (Math|Rotator|MakeRotator (Math|Float|ClampAngle (.roll _output_get) -45.0 45.0) (.pitch _output_get) (Math|Float|ClampAngle (.yaw _output_get) -1.8e+02 0.0)) false false))

(event EventBeginPlay
  (Variables|Default|SetCurrentRotationCamera (Transformation|GetWorldRotation (Variables|Default|GetCamera))))

(event Collision|EventActorBeginOverlap
  (params (OtherActor :type Actor%20Object%20Reference)))

(event EventTick
  (params (DeltaSeconds :type Float%20%28single-precision%29)))

(fn ConstructionScript)
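; BP_Card is an interactable card item that tints its Cube mesh red, blue or green according to its ColorCard value.
; On BeginPlay it creates a dynamic instance of M_BaseMat with a faint emissive level and passes it to CreateDynamicMaterial.
; That function sets the base and emissive colors to the matching value and applies the material to the mesh.
; The Sphere overlap events are empty, so no pickup logic runs here.
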(event OnComponentBeginOverlap(Sphere)
  (params (OverlappedComponent :type Primitive%20Component%20Object%20Reference) (OtherActor :type Actor%20Object%20Reference) (OtherComp :type Primitive%20Component%20Object%20Reference) (OtherBodyIndex :type Integer) (bFromSweep :type Boolean) (SweepResult :type Hit%20Result%20Structure%20%28by%20ref%29)))

(event OnComponentEndOverlap(Sphere)
  (params (OverlappedComponent :type Primitive%20Component%20Object%20Reference) (OtherActor :type Actor%20Object%20Reference) (OtherComp :type Primitive%20Component%20Object%20Reference) (OtherBodyIndex :type Integer)))

(event EventBeginPlay
  (bind _returnvalue (Rendering|Material|CreateDynamicMaterialInstance "/Game/Materials/M_BaseMat.M_BaseMat" "None" "None" :!class /Script/Engine.KismetMaterialLibrary))
  (Rendering|Material|SetScalarParameterValue _returnvalue "Emissive" 0.05 :!class /Script/Engine.MaterialInstanceDynamic)
  (CallFunction|CreateDynamicMaterial _returnvalue (Variables|Default|GetCube)))

(event Collision|EventActorBeginOverlap
  (params (OtherActor :type Actor%20Object%20Reference)))

(event EventTick
  (params (DeltaSeconds :type Float%20%28single-precision%29)))

(fn ConstructionScript)

(fn CreateDynamicMaterial
  (params (Material%20Instance :type Material%20Instance%20Dynamic%20Object%20Reference) (Mesh :type Static%20Mesh%20Component%20Object%20Reference))
  (bind _redvalue (Variables|Default|GetRedValue))
  (bind _blue_value (Variables|Default|GetBlue%20Value))
  (bind _green_value (Variables|Default|GetGreen%20Value))
  (switch Utilities|FlowControl|Switch|SwitchonEColorDoor (Variables|Default|GetColorCard)
    (:NewEnumerator0
      (Rendering|Material|SetVectorParameterValue Material%20Instance "Color" _redvalue :!class /Script/Engine.MaterialInstanceDynamic)
      (Rendering|Material|SetVectorParameterValue Material%20Instance "ColorEmissive" _redvalue :!class /Script/Engine.MaterialInstanceDynamic))
    (:NewEnumerator1
      (Rendering|Material|SetVectorParameterValue Material%20Instance "Color" _blue_value :!class /Script/Engine.MaterialInstanceDynamic)
      (Rendering|Material|SetVectorParameterValue Material%20Instance "ColorEmissive" _blue_value :!class /Script/Engine.MaterialInstanceDynamic))
    (:NewEnumerator2
      (Rendering|Material|SetVectorParameterValue Material%20Instance "Color" _green_value :!class /Script/Engine.MaterialInstanceDynamic)
      (Rendering|Material|SetVectorParameterValue Material%20Instance "ColorEmissive" _green_value :!class /Script/Engine.MaterialInstanceDynamic)))
  (Rendering|Material|SetMaterial Mesh 0 Material%20Instance))
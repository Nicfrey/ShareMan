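; BPC_Timer is a reusable timer component, filed under interactable items, that tracks elapsed time and reports it as progress.
; Once started, Tick adds or subtracts delta seconds based on a direction flag that events can flip, with no clamping or completion event.
; Restart zeroes and stops the timer in counting-up mode, and GetPercentageTimer returns the current value divided by Time as an unclamped ratio.
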(event Custom|RestartTimer
  (Variables|Default|SetcurrentTimer 0.0)
  (Variables|Default|Setstarted false)
  (Variables|Default|SetisDecreasingTime false))

(event Custom|StartTimer
  (Variables|Default|Setstarted true))

(event Custom|DecreasingTimer
  (Variables|Default|SetisDecreasingTime true))

(event Custom|IncreasingTimer
  (Variables|Default|SetisDecreasingTime false))

(event EventBeginPlay)

(event EventTick
  (params (DeltaSeconds :type Float%20%28single-precision%29))
  ;[1 1 1] Check if the timer is started or not
  (if (Variables|Default|Getstarted)
    (if (Variables|Default|GetisDecreasingTime)
      ;[1 1 1] Decreasing Timer
      (Variables|Default|SetcurrentTimer (- (Variables|Default|GetcurrentTimer) DeltaSeconds))
      (else
        ;[1 1 1] Increasing Timer
        (Variables|Default|SetcurrentTimer (+ DeltaSeconds (Variables|Default|GetcurrentTimer)))))))

(fn GetPercentageTimer
  (return (/ (Variables|Default|GetcurrentTimer) (Variables|Default|GetTime))))
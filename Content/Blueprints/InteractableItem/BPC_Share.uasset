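; BPC_Share is an interactable share pickup that adds to the share count tracked by BP_MyGameMode.
; On Interact, it adds its Amount to the game mode's NbShareGot and prints the new total.
; A Got flag limits the reward to a single interaction.
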(event EventBeginPlay)

(event EventTick
  (params (DeltaSeconds :type Float%20%28single-precision%29)))

(event EventInteract
  (bind _returnvalue (Game|GetGameMode))
  (bind _asbp_my_game_mode (Utilities|Casting|CastToBP_MyGameMode _returnvalue))
  (if (not (Variables|Default|GetGot))
    (bind _output_get (Variables|/Game/Blueprints/BP_MyGameMode.BP_MyGameMode_C|SetnbShareGot _asbp_my_game_mode (+ (Variables|Default|Getamount) (Variables|/Game/Blueprints/BP_MyGameMode.BP_MyGameMode_C|GetnbShareGot _asbp_my_game_mode))))
    (Development|PrintString (Utilities|String|ToString(Integer) _output_get))
    (Variables|Default|SetGot true)))
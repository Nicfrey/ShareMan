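; BP_MonitorsCamera is an interactable monitor station that lets the player view and cycle through the level's cameras.
; It gathers every BP_Camera at BeginPlay, and its Box overlap registers or clears it as the player character's CurrentInteractCameras.
; Interact makes player controller 0 possess the last-seen camera, rather than blending view targets.
; NextCamera and PreviousCamera step that index with wraparound, possess the new camera and print the index.
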(event OnComponentBeginOverlap(Box)
  (params (OverlappedComponent :type Primitive%20Component%20Object%20Reference) (OtherActor :type Actor%20Object%20Reference) (OtherComp :type Primitive%20Component%20Object%20Reference) (OtherBodyIndex :type Integer) (bFromSweep :type Boolean) (SweepResult :type Hit%20Result%20Structure%20%28by%20ref%29))
  (bind _asbp_player_character (Utilities|Casting|CastToBP_PlayerCharacter OtherActor))
  (Variables|/Game/Blueprints/Player/BP_PlayerCharacter.BP_PlayerCharacter_C|SetCurrentInteractCameras _asbp_player_character self))

(event OnComponentEndOverlap(Box)
  (params (OverlappedComponent :type Primitive%20Component%20Object%20Reference) (OtherActor :type Actor%20Object%20Reference) (OtherComp :type Primitive%20Component%20Object%20Reference) (OtherBodyIndex :type Integer))
  (bind _asbp_player_character (Utilities|Casting|CastToBP_PlayerCharacter OtherActor))
  (Variables|/Game/Blueprints/Player/BP_PlayerCharacter.BP_PlayerCharacter_C|SetCurrentInteractCameras _asbp_player_character 0))

(event Custom|NextCamera
  (bind _result (Math|Integer|IncrementInt (Variables|Default|GetLastSeenCameraIndex))
    (:%20%20
      (if (>= _result (Utilities|Array|Length (Variables|Default|GetCameras)))
        (Variables|Default|SetLastSeenCameraIndex 0))
      (Pawn|Possess (Game|GetPlayerController 0) (Utilities|Array|Get(acopy) (Variables|Default|GetCameras) (Variables|Default|GetLastSeenCameraIndex)))
      (Development|PrintString (Utilities|String|ToString(Integer) (Variables|Default|GetLastSeenCameraIndex))))))

(event Custom|PreviousCamera
  (bind _result (Math|Integer|DecrementInt (Variables|Default|GetLastSeenCameraIndex))
    (:%20%20
      (if (< _result 0)
        (Variables|Default|SetLastSeenCameraIndex (- (Utilities|Array|Length (Variables|Default|GetCameras)) 1)))
      (Pawn|Possess (Game|GetPlayerController 0) (Utilities|Array|Get(acopy) (Variables|Default|GetCameras) (Variables|Default|GetLastSeenCameraIndex)))
      (Development|PrintString (Utilities|String|ToString(Integer) (Variables|Default|GetLastSeenCameraIndex))))))

(event EventBeginPlay
  (bind _outactors (Actor|GetAllActorsOfClass "/Game/Blueprints/InteractableItem/BP_Camera.BP_Camera_C"))
  (Variables|Default|SetCameras _outactors))

(event Collision|EventActorBeginOverlap
  (params (OtherActor :type Actor%20Object%20Reference)))

(event EventTick
  (params (DeltaSeconds :type Float%20%28single-precision%29)))

(event EventInteract
  (Pawn|Possess (Game|GetPlayerController 0) (Utilities|Array|Get(acopy) (Variables|Default|GetCameras) (Variables|Default|GetLastSeenCameraIndex))))

(fn ConstructionScript)
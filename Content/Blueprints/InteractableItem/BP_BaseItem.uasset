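; Base interactable item that raises the boss's anger when it moves fast after being hit by the player.
; Box hit events set a flag when the player hits the item and clear it when an enemy does.
; While the flag is set, Tick runs a short Delay, then compares mesh velocity to a threshold and calls UpdateAngryLevel on the boss found by class.
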(event OnComponentHit(Box)
  (params (HitComponent :type Primitive%20Component%20Object%20Reference) (OtherActor :type Actor%20Object%20Reference) (OtherComp :type Primitive%20Component%20Object%20Reference) (NormalImpulse :type Vector :default "0, 0, 0") (Hit :type Hit%20Result%20Structure%20%28by%20ref%29))
  (Utilities|FlowControl|Sequence
    (:then_0
      (Utilities|Casting|CastToBP_PlayerCharacter OtherActor)
      (Variables|Default|SetLastHitIsPlayer true))
    (:then_1
      (Utilities|Casting|CastToBP_EnemyCharacter OtherActor)
      (Variables|Default|SetLastHitIsPlayer false))))

(event EventBeginPlay)

(event Collision|EventActorBeginOverlap
  (params (OtherActor :type Actor%20Object%20Reference)))

(event EventTick
  (params (DeltaSeconds :type Float%20%28single-precision%29))
  (if (Variables|Default|GetLastHitIsPlayer)
    (Utilities|FlowControl|Delay 0.7)
    (if (>= (Math|Vector|VectorLength (Transformation|GetComponentVelocity (Variables|Default|GetStaticMesh))) (Variables|Default|GetMaxVelocityBeforeDamage))
      (bind _returnvalue (Actor|GetActorOfClass "/Game/Blueprints/Enemies/BP_BossCharacter.BP_BossCharacter_C"))
      (Default|UpdateAngryLevel _returnvalue 2.0))))

(fn ConstructionScript)
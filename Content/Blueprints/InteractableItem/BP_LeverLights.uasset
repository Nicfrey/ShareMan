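; Interactable lever that switches all level lamps and sky intensity on or off.
; Interact starts a timed rotation driven from Tick; on completion it updates BP_Lamp actors, the game mode sky and every enemy's IsLightOn blackboard key.
; Box overlap registers the lever with the player, or starts a timer for the boss to flip it back on when off.
; TurnTheLightOn forces the lit state without animating; TurnTheLights is an unfinished stub.
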(event OnComponentBeginOverlap(Box)
  (params (OverlappedComponent :type Primitive%20Component%20Object%20Reference) (OtherActor :type Actor%20Object%20Reference) (OtherComp :type Primitive%20Component%20Object%20Reference) (OtherBodyIndex :type Integer) (bFromSweep :type Boolean) (SweepResult :type Hit%20Result%20Structure%20%28by%20ref%29))
  (Utilities|FlowControl|Sequence
    (:then_0
      (bind _asbp_player_character (Utilities|Casting|CastToBP_PlayerCharacter OtherActor))
      (Variables|/Game/Blueprints/Player/BP_PlayerCharacter.BP_PlayerCharacter_C|SetCurrentInteractLever _asbp_player_character self)
      (Development|PrintString "Can turn light "))
    (:then_1
      (Utilities|Casting|CastToBP_BossCharacter OtherActor)
      (if (Utilities|Enum|Equal(Enum) (Variables|Default|Getstatus) "NewEnumerator2")
        (if (not (Variables|/Game/Blueprints/InteractableItem/BPC_Timer.BPC_Timer_C|Getstarted (Variables|Default|GetTimerBoss)))
          (Default|StartTimer (Variables|Default|GetTimerBoss)))))))

(event OnComponentEndOverlap(Box)
  (params (OverlappedComponent :type Primitive%20Component%20Object%20Reference) (OtherActor :type Actor%20Object%20Reference) (OtherComp :type Primitive%20Component%20Object%20Reference) (OtherBodyIndex :type Integer))
  (bind _asbp_player_character (Utilities|Casting|CastToBP_PlayerCharacter OtherActor))
  (Variables|/Game/Blueprints/Player/BP_PlayerCharacter.BP_PlayerCharacter_C|SetCurrentInteractLever _asbp_player_character 0)
  (Development|PrintString "Stop turn light"))

(event Custom|Rotate
  (bind _timerrotation (Variables|Default|GetTimerRotation))
  (bind _lever (Variables|Default|GetLever))
  (bind _percentage (Default|GetPercentageTimer _timerrotation))
  (bind _returnvalue (>= _percentage 1.0))
  ;[1 1 1] Rotate the lever
  ;;[1 1 1] Check if the current rotation is on or off
  (switch Utilities|FlowControl|Switch|SwitchonEStatus_Lever (Variables|Default|Getstatus)
    (:NewEnumerator1
      ;;[1 1 1] Rotate to the correct angle the lever
      (Transformation|SetRelativeRotation _lever (Math|Rotator|Lerp(Rotator) (Variables|Default|GetCurrentRotation) (Math|Rotator|MakeRotator (Variables|Default|GetAngleOff) 0.0 0.0) (Default|GetPercentageTimer (Variables|Default|GetTimerRotation)) true) false false)
      (if _returnvalue
        (Variables|Default|Setstatus "NewEnumerator2")
        (Variables|Default|SetCurrentRotation (Math|Rotator|Lerp(Rotator) (Variables|Default|GetCurrentRotation) (Math|Rotator|MakeRotator (Variables|Default|GetAngleOff) 0.0 0.0) (Default|GetPercentageTimer (Variables|Default|GetTimerRotation)) true))
        (bind _asbp_my_game_mode (Utilities|Casting|CastToBP_MyGameMode (Game|GetGameMode)))
        (Default|ChangeSkyIntensity _asbp_my_game_mode false)
        (Development|PrintString "Off")
        ;[1 1 1] Turn the light off or on
        (bind _outactors (Actor|GetAllActorsOfClass "/Game/Blueprints/InteractableItem/BP_Lamp.BP_Lamp_C" :!label _label))
        (for _array_element _outactors
          (Default|TurntheLight _array_element (Utilities|Enum|Equal(Enum) (Variables|Default|Getstatus) "NewEnumerator0"))
          ;[1 1 1] Change blackboard value for Enemies
          (bind _outactors_2 (Actor|GetAllActorsOfClass "/Game/Blueprints/Enemies/BP_EnemyCharacter.BP_EnemyCharacter_C"))
          (for _array_element_2 _outactors_2
            (AI|Components|Blackboard|SetValueasBool (AI|GetBlackboard (AI|GetAIController _array_element_2)) (Utilities|Name|MakeLiteralName "IsLightOn") (CallFunction|IsLighton))))
        (Default|ResetTimer (Variables|Default|GetTimerRotation))))
    (:NewEnumerator3
      (Transformation|SetRelativeRotation _lever (Math|Rotator|Lerp(Rotator) (Variables|Default|GetCurrentRotation) (Math|Rotator|MakeRotator (Variables|Default|GetAngleOn) 0.0 0.0) (Default|GetPercentageTimer (Variables|Default|GetTimerRotation)) true) false false)
      (if _returnvalue
        (Variables|Default|Setstatus "NewEnumerator0")
        (Variables|Default|SetCurrentRotation (Math|Rotator|Lerp(Rotator) (Variables|Default|GetCurrentRotation) (Math|Rotator|MakeRotator (Variables|Default|GetAngleOn) 0.0 0.0) (Default|GetPercentageTimer (Variables|Default|GetTimerRotation)) true))
        (bind _asbp_my_game_mode_2 (Utilities|Casting|CastToBP_MyGameMode (Game|GetGameMode)))
        (Default|ChangeSkyIntensity _asbp_my_game_mode_2 true)
        (Development|PrintString "On")
        (goto _label)))))

(event EventBeginPlay
  (Transformation|SetRelativeRotation (Variables|Default|GetLever) (Variables|Default|GetCurrentRotation) false false))

(event Collision|EventActorBeginOverlap
  (params (OtherActor :type Actor%20Object%20Reference)))

(event EventTick
  (params (DeltaSeconds :type Float%20%28single-precision%29))
  (CallFunction|Rotate)
  (if (>= (Default|GetPercentageTimer (Variables|Default|GetTimerBoss)) 1.0)
    (Default|ResetTimer (Variables|Default|GetTimerBoss))
    (CallFunction|Interact)))

(event EventInteract
  (switch Utilities|FlowControl|Switch|SwitchonEStatus_Lever (Variables|Default|Getstatus)
    (:NewEnumerator0
      (Variables|Default|Setstatus "NewEnumerator1")
      (Development|PrintString "TurningOff"))
    (:NewEnumerator2
      (Variables|Default|Setstatus "NewEnumerator3")
      (Development|PrintString "TurningOn")))
  (Default|StartTimer (Variables|Default|GetTimerRotation)))

(fn ConstructionScript)

(fn TurntheLights
  (params (lamps :type Array%20of%20BP%20Lamp%20Object%20References))
  (switch Utilities|FlowControl|Switch|SwitchonEStatus_Lever (Variables|Default|Getstatus)
    (:NewEnumerator0
      (for _array_element lamps
        _))
    (:NewEnumerator2
      (for _array_element_2 lamps
        _))))

(fn IsLighton
  (return (Utilities|Enum|Equal(Enum) (Variables|Default|Getstatus) "NewEnumerator0")))

(fn GetPositionLever
  (return (Transformation|GetWorldLocation (Variables|Default|GetPositionLever))))

(fn TurntheLighton
  (Variables|Default|Setstatus "NewEnumerator0")
  ;[1 1 1] Change blackboard value for Enemies
  (bind _outactors (Actor|GetAllActorsOfClass "/Game/Blueprints/Enemies/BP_EnemyCharacter.BP_EnemyCharacter_C"))
  (for _array_element _outactors
    (AI|Components|Blackboard|SetValueasBool (AI|GetBlackboard (AI|GetAIController _array_element)) (Utilities|Name|MakeLiteralName "IsLightOn") (CallFunction|IsLighton))
    ;[1 1 1] Turn the light off or on
    (bind _outactors_2 (Actor|GetAllActorsOfClass "/Game/Blueprints/InteractableItem/BP_Lamp.BP_Lamp_C"))
    (for _array_element_2 _outactors_2
      (Default|TurntheLight _array_element_2 true)
      (bind _asbp_my_game_mode (Utilities|Casting|CastToBP_MyGameMode (Game|GetGameMode)))
      (Default|ChangeSkyIntensity _asbp_my_game_mode true))
    (Default|ResetTimer (Variables|Default|GetTimerRotation))))
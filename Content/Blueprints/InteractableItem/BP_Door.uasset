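; BP_Door is a colored door that swings open for enemies, and for other actors such as the player only if it is white or unlocked through OpenDoor.
; A color component tints a dynamic material on the mesh and supplies the color check.
; Box overlaps count enemies and start or reverse a timer component.
; Tick maps timer progress to door yaw, while collision switches between ignore and block.
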(event OnComponentBeginOverlap(Box)
  (params (OverlappedComponent :type Primitive%20Component%20Object%20Reference) (OtherActor :type Actor%20Object%20Reference) (OtherComp :type Primitive%20Component%20Object%20Reference) (OtherBodyIndex :type Integer) (bFromSweep :type Boolean) (SweepResult :type Hit%20Result%20Structure%20%28by%20ref%29))
  (bind _timeopening (Variables|Default|GetTimeOpening))
  (Utilities|Casting|CastToBP_EnemyCharacter OtherActor
    (:then
      (Math|Integer|IncrementInt (Variables|Default|GetEnemiesOnDoor)
        (:%20%20
          (if (not (Variables|/Game/Blueprints/InteractableItem/BPC_Timer.BPC_Timer_C|Getstarted _timeopening)) :!label _label
            (Default|StartTimer _timeopening)
            (Collision|SetCollisionResponsetoAllChannels (Variables|Default|GetDoor) "ECR_Ignore")))))
    (:CastFailed
      (if (Variables|Default|GetLetPlayerPass)
        (goto _label)))))

(event OnComponentEndOverlap(Box)
  (params (OverlappedComponent :type Primitive%20Component%20Object%20Reference) (OtherActor :type Actor%20Object%20Reference) (OtherComp :type Primitive%20Component%20Object%20Reference) (OtherBodyIndex :type Integer))
  (Utilities|Casting|CastToBP_Door OtherActor
    (:CastFailed
      (Utilities|Casting|CastToBP_EnemyCharacter OtherActor
        (:then
          (bind _result (Math|Integer|DecrementInt (Variables|Default|GetEnemiesOnDoor))
            (:%20%20
              (if (<= _result 0)
                (Default|DecreasingTimer (Variables|Default|GetTimeOpening) :!label _label)
                (Collision|SetCollisionResponsetoAllChannels (Variables|Default|GetDoor) "ECR_Block")))))
        (:CastFailed
          (if (Variables|Default|GetLetPlayerPass)
            (goto _label)))))))

(event Custom|OpenDoor
  (Variables|Default|SetLetPlayerPass true))

(event EventBeginPlay
  (bind _door (Variables|Default|GetDoor))
  ;[1 1 1] Check if the door is white or not
  (Variables|Default|SetLetPlayerPass (Utilities|Enum|Equal(Enum) (Variables|/Game/Blueprints/InteractableItem/BPC_ColorDoor.BPC_ColorDoor_C|GetColor (Variables|Default|GetBPC_ColorDoor)) "NewEnumerator3"))
  ;[1 1 1] Apply the correct color of the door
  (bind _returnvalue (Rendering|Material|CreateDynamicMaterialInstance "/Game/Materials/M_BaseMat.M_BaseMat" "None" "None" :!class /Script/Engine.KismetMaterialLibrary))
  (Default|ApplyColortoMaterial (Variables|Default|GetBPC_ColorDoor) _door _returnvalue 1)
  (Rendering|Material|SetMaterial _door 1 _returnvalue))

(event Collision|EventActorBeginOverlap
  (params (OtherActor :type Actor%20Object%20Reference)))

(event EventTick
  (params (DeltaSeconds :type Float%20%28single-precision%29))
  (bind _timeopening (Variables|Default|GetTimeOpening))
  (if (Variables|/Game/Blueprints/InteractableItem/BPC_Timer.BPC_Timer_C|Getstarted _timeopening)
    (Transformation|SetRelativeRotation (Variables|Default|GetDoor) (Math|Rotator|MakeRotator 0.0 0.0 (Math|Float|Lerp (Variables|Default|GetMinAngleRotation) (Variables|Default|GetMaxAngleRotation) (Math|Float|Clamp(Float) (Default|GetPercentageTimer _timeopening)))) false false)
    (Collision|SetCollisionResponsetoAllChannels (Variables|Default|GetDoor) "ECR_Ignore")))

(fn ConstructionScript)

(fn GetColor
  (return (Variables|/Game/Blueprints/InteractableItem/BPC_ColorDoor.BPC_ColorDoor_C|GetColor (Variables|Default|GetBPC_ColorDoor))))
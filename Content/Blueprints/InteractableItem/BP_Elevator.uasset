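; BP_Elevator is an interactable elevator whose Interact event calls GameOver on BP_MyGameMode.
; A box overlap passes the player's CanLeave result to CanLeaveInsideElevator and registers this elevator as the player's CurrentElevator, clearing it on exit.
; The EmergencyLight event switches the point light between on and off colors.
; GetPosition returns the world location of the PositionSpawn component.
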(event OnComponentBeginOverlap(Box)
  (params (OverlappedComponent :type Primitive%20Component%20Object%20Reference) (OtherActor :type Actor%20Object%20Reference) (OtherComp :type Primitive%20Component%20Object%20Reference) (OtherBodyIndex :type Integer) (bFromSweep :type Boolean) (SweepResult :type Hit%20Result%20Structure%20%28by%20ref%29))
  (bind _asbp_player_character (Utilities|Casting|CastToBP_PlayerCharacter OtherActor))
  (bind _canleave (Default|CanLeave _asbp_player_character))
  (Default|CanLeaveInsideElevator _asbp_player_character _canleave)
  (Variables|/Game/Blueprints/Player/BP_PlayerCharacter.BP_PlayerCharacter_C|SetCurrentElevator _asbp_player_character self))

(event OnComponentEndOverlap(Box)
  (params (OverlappedComponent :type Primitive%20Component%20Object%20Reference) (OtherActor :type Actor%20Object%20Reference) (OtherComp :type Primitive%20Component%20Object%20Reference) (OtherBodyIndex :type Integer))
  (bind _asbp_player_character (Utilities|Casting|CastToBP_PlayerCharacter OtherActor))
  (Variables|/Game/Blueprints/Player/BP_PlayerCharacter.BP_PlayerCharacter_C|SetCurrentElevator _asbp_player_character 0))

(event Custom|EmergencyLight
  (params (Light%20on :type Boolean))
  (bind _pointlight (Variables|Default|GetPointLight))
  (if Light%20on
    (Rendering|Components|Light|SetLightColor _pointlight (Variables|Default|GetLightOnColor) true)
    (else
      (Rendering|Components|Light|SetLightColor _pointlight (Variables|Default|GetLightOffColor) true))))

(event EventBeginPlay)

(event Collision|EventActorBeginOverlap
  (params (OtherActor :type Actor%20Object%20Reference)))

(event EventTick
  (params (DeltaSeconds :type Float%20%28single-precision%29)))

(event EventInteract
  (bind _asbp_my_game_mode (Utilities|Casting|CastToBP_MyGameMode (Game|GetGameMode)))
  (Default|GameOver _asbp_my_game_mode))

(fn ConstructionScript)

(fn GetPosition
  (return (Transformation|GetWorldLocation (Variables|Default|GetPositionSpawn))))